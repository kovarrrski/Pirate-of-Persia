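; 2D flipbook sword projectile that damages shark enemies or sticks into walls as a platform the hero can jump on.
; On a box hit, it plays the embedded animation once, snaps the flipbook to a corrective offset and sets the box to block Pawns.
; On overlapping a BP_Shark, it calls ReceiveAttack with fixed damage and destroys itself.
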(event `self.Box.OnComponentHit`
  (params (HitComponent :type "PrimitiveComponent Object Reference") (OtherActor :type "Actor Object Reference") (OtherComp :type "PrimitiveComponent Object Reference") (NormalImpulse :type "Vector Structure") (Hit :type "HitResult Structure (by ref)"))
  ;[1 1 1] Play Sword's Stucked Anim (FB)
  (`PaperFlipbookComponent.SetFlipbook` (`self.SwordFlipbook`) "/Game/PaperAssets/Sword/Captain__Sword_Embedded.Captain__Sword_Embedded")
  ;[1 1 1] Play only once Anim (FB)
  (`PaperFlipbookComponent.SetLooping` (`self.SwordFlipbook`) false)
  ;[1 1 1] Set FB's new location (-30X), because flipbook's asset is not aligned perfectly. Now it visible perfectly, befor - a half of the Sword was hide.
  (`SceneComponent.K2_SetRelativeLocation` (`self.SwordFlipbook`) (`SceneComponent.RelativeLocation` (`self.EmbeddedPos`)) false false)
  ;[1 1 1] Change SwordBox Collision on Block, after stucking to the Wall. So Hero can jump on it.
  (`PrimitiveComponent.SetCollisionResponseToChannel` (`self.Box`) "ECC_Pawn" "ECR_Block"))

(event `self.Box.OnComponentBeginOverlap`
  (params (OverlappedComponent :type "PrimitiveComponent Object Reference") (OtherActor :type "Actor Object Reference") (OtherComp :type "PrimitiveComponent Object Reference") (OtherBodyIndex :type Integer) (bFromSweep :type Boolean) (SweepResult :type "HitResult Structure (by ref)"))
  ;[1 1 1] If Sword Overlapped an Enemy, it makes 50 damage to the Enemy and self-destroys after
  (bind _asbp_shark (cast `/Game/Blueprints/Characters/Shark/BP_Shark` OtherActor))
  (`/Game/Blueprints/Characters/BP_ActionChar.ReceiveAttack` _asbp_shark 50.0)
  (`self.K2_DestroyActor`))

(fn `UserConstructionScript`)