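; AI controller for enemies that runs their behavior tree and temporarily sets the player's captain as attack target on BeginPlay.
; On possess, it binds to the ActionChar's stun event and mirrors that state, like the target, into the Blackboard.
; Each tick it sets a focal point toward the target along the X axis only, or straight ahead when the character cannot act or has no target.
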(event `self.ReceiveBeginPlay`
  ;[1 1 1] Connect BB and BT with AIC
  (`self.UseBlackboard` "/Game/Blueprints/AI/BB_Enemy.BB_Enemy")
  (`self.RunBehaviorTree` "/Game/Blueprints/AI/BT_Enemy.BT_Enemy")
  ;[1 1 1] AI looks for the player snd set it as target. Temporary Aggro
  (bind _asbp_captain (cast `/Game/Blueprints/Characters/Captain/BP_Captain` (`GameplayStatics.GetPlayerPawn` 0)))
  (`self.SetAttackTarget` _asbp_captain))

(event `self.ReceiveTick`
  (params (DeltaSeconds :type "Float (single-precision)"))
  (`self.SetFocusDirection`))

(event `self.ReceivePossess`
  (params (PossessedPawn :type "Pawn Object Reference"))
  (bind _asbp_action_char (cast `/Game/Blueprints/Characters/BP_ActionChar` PossessedPawn))
  ;[1 1 1] When Char Change StunState (informed via event), BB gets information about Stuns
  (bind _output_get (set `self.ActionChar` _asbp_action_char))
  (add `/Game/Blueprints/Characters/BP_ActionChar.StunStateChanged` _output_get (delegate `OnStunStateChanged`)))

(event `OnStunStateChanged`
  (params (IsStunned :type Boolean))
  ;[1 1 1] When Char Change StunState (informed via event), BB gets information about Stuns
  ;;[1 1 1] Setting of Bool Stunned value into the BB by Key
  (`BlackboardComponent.SetValueAsBool` (`self.Blackboard`) (`self.IsStunnedKey`) IsStunned))

(fn `SetAttackTarget`
  (params (AttackTarget :type "/Game/Blueprints/Characters/Captain/BP_Captain Object Reference"))
  ;[1 1 1] Pass Attack Target to set in the BB
  (`BlackboardComponent.SetValueAsObject` (`self.Blackboard`) (`self.AttackTargetKey`) (`local.AttackTarget`))
  (set `self.Attack Target` (`local.AttackTarget`)))

(fn `SetFocusDirection`
  (bind _actionchar (`self.ActionChar`))
  (bind _returnvalue_x (`KismetMathLibrary.BreakVector` (`KismetMathLibrary.GetForwardVector` (`KismetMathLibrary.FindLookAtRotation` (`self.K2_GetActorLocation` (`self.ActionChar`)) (`self.K2_GetActorLocation` (`self.Attack Target`))))))
  (`/Engine/EditorBlueprintResources/StandardMacros.IsValid` (`self.Attack Target`)
    (:`Is Valid`
      (if (`/Game/Blueprints/Characters/BP_ActionChar.CanAct` (`self.ActionChar`))
        ;[1 1 1] Char's Rotation to the target
        (`self.K2_SetFocalPoint` (+ (`self.K2_GetActorLocation` (`self.ActionChar`)) (`KismetMathLibrary.MakeVector` _returnvalue_x)))
        (else
          ;[1 1 1] Enemy looks to Hero anyway, if he stunned, attacking or have no Target for chasing
          (`self.K2_SetFocalPoint` (+ (`self.K2_GetActorLocation` _actionchar) (`self.GetActorForwardVector` _actionchar)) :!label _label))))
    (:`Is Not Valid`
      (goto _label))))

(fn `UserConstructionScript`)