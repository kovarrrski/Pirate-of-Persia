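; BP_ActionChar is an action character with health, faction-based melee hit detection and a stun reaction.
; Its Hitbox starts disabled, is switched through SetHitboxCollision, and deals fixed damage to overlapping BP_ActionChar actors of another faction.
; ReceiveAttack subtracts health and, if any remains, sets IsStunned, jumps the animation instance to its stunned node and starts a stun-length timer.
; Reaching zero health triggers no further logic here.
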(event `self.ReceiveBeginPlay`
  (`self.SetHitboxCollision` false)
  ;[1 1 1] Max Health at the Start as Current Health
  (set `self.CurrentHealth` (`self.MaxHealth`)))

(event `self.Hitbox.OnComponentBeginOverlap`
  (params (OverlappedComponent :type "PrimitiveComponent Object Reference") (OtherActor :type "Actor Object Reference") (OtherComp :type "PrimitiveComponent Object Reference") (OtherBodyIndex :type Integer) (bFromSweep :type Boolean) (SweepResult :type "HitResult Structure (by ref)"))
  ;[1 1 1] Overlap with Char, Shark = Attack . Hero faction = 0, Enemy=1. Attack executes only on Enemies  (with fraction 1)
  (bind _asbp_action_char (cast `/Game/Blueprints/Characters/BP_ActionChar` OtherActor))
  (if (!= (`/Game/Blueprints/Characters/BP_ActionChar.Faction` _asbp_action_char) (`self.Faction`))
    (`self.ReceiveAttack` _asbp_action_char 25.0)))

(fn `ClearStun`
  (set `self.IsStunned` false))

(fn `ReceiveAttack`
  (params (Damage :type "Float (double-precision)" :default 25.0))
  ;[1 1 1] - Damage
  (set `self.CurrentHealth` (- (`self.CurrentHealth`) Damage))
  (if (not (<= (`self.CurrentHealth`) 0.0))
    ;[1 1 1] "Jumps" Conection from Locomotion. Play Anim of Stuned when ReceivingAttack
    (set `self.IsStunned` true)
    (`PaperZDAnimInstance.JumpToNode` (`self.GetAnimInstance`) "JumpStunned" "None")
    ;[1 1 1] Event f ClearStun after 0.5sec of Stun Anim
    (`KismetSystemLibrary.K2_SetTimerDelegate` (`|CreateDelegate` :!event `ClearStun`) (`self.StunLength`))))

(fn `SetHitboxCollision`
  (params (SetActive :type Boolean))
  ;[1 1 1] Activator of the Collision of hitbox - Switcher
  (if SetActive
    (`PrimitiveComponent.SetCollisionEnabled` (`self.Hitbox`) "QueryOnly")
    (else
      (`PrimitiveComponent.SetCollisionEnabled` (`self.Hitbox`) "NoCollision"))))

(fn `UserConstructionScript`)